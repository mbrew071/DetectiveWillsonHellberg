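; Newspaper boy NPC that shouts while the player is nearby, driven by a narration graph.
; Its Box overlap starts BP_EgDialogueGraph1 on the GraphNarrationTarget with itself as actor when a player-tagged actor enters, and ends it as PlayerIsAway on exit.
; Ending an interaction restarts the shouting.
; A delayed check for a player already inside the box at game start exists but is never run.
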(event OnComponentBeginOverlap(Box)
  (params (OverlappedComponent :type Primitive%20Component%20Object%20Reference) (OtherActor :type Actor%20Object%20Reference) (OtherComp :type Primitive%20Component%20Object%20Reference) (OtherBodyIndex :type Integer) (bFromSweep :type Boolean) (SweepResult :type Hit%20Result%20Structure%20%28by%20ref%29))
  ;[0 0.000581 0.005] Player got near to this npc. Therefore Npc will start shouting
  (if (Actor|ActorHasTag OtherActor "Actor.Character.Player")
    (Class|GraphNarrationTarget|BeginNarrationGraph (Variables|Default|GetGraphNarrationTarget) (Utilities|Array|MakeArray self) "/SimpleNarration/DialogueGraphs/BP_EgDialogueGraph1.BP_EgDialogueGraph1_C")))

(event OnComponentEndOverlap(Box)
  (params (OverlappedComponent :type Primitive%20Component%20Object%20Reference) (OtherActor :type Actor%20Object%20Reference) (OtherComp :type Primitive%20Component%20Object%20Reference) (OtherBodyIndex :type Integer))
  ;[0 0.000581 0.005] Stop shouting because player is too far away
  (if (Actor|ActorHasTag OtherActor "Actor.Character.Player")
    (Class|GraphNarrationTarget|EndNarrationGraph (Variables|Default|GetGraphNarrationTarget) "(TagName=\"GraphNarration.FailureReason.PlayerIsAway\")")))

(event Custom|Start%20Shouting
  ;[0 0.000581 0.005] Player got near to this npc. Therefore Npc will start shouting
  (Class|GraphNarrationTarget|BeginNarrationGraph (Variables|Default|GetGraphNarrationTarget) (Utilities|Array|MakeArray self) "/SimpleNarration/DialogueGraphs/BP_EgDialogueGraph1.BP_EgDialogueGraph1_C"))

(event EventBeginPlay
  (|CallParentFunction))

(event Collision|EventActorBeginOverlap
  (params (OtherActor :type Actor%20Object%20Reference))
  (|CallParentFunction OtherActor) ; This node is disabled and will not be called.\nDrag off pins to build functionality.
)

(event EventTick
  (params (DeltaSeconds :type Float%20%28single-precision%29))
  (|CallParentFunction DeltaSeconds) ; This node is disabled and will not be called.\nDrag off pins to build functionality.
)

(fn ConstructionScript
  (|CallParentFunction))

(fn OnInteractionEnd
  (params (InteractionTag :type Gameplay%20Tag%20Structure))
  (CallFunction|StartShouting))