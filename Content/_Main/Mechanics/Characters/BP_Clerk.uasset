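; BP_Clerk is a clerk NPC that greets the player and offers dialogue through narration graphs.
; A player-tagged actor entering its Box starts the BP_ClerkGreeting graph, which serves as the clerk's shouting.
; Beginning a ClickInteract interaction starts BP_ClerkDialogue, with the clerk as narration actor.
; OnInteractionEnd calls StartShouting to run the greeting graph again.
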(event OnComponentBeginOverlap(Box)
  (params (OverlappedComponent :type Primitive%20Component%20Object%20Reference) (OtherActor :type Actor%20Object%20Reference) (OtherComp :type Primitive%20Component%20Object%20Reference) (OtherBodyIndex :type Integer) (bFromSweep :type Boolean) (SweepResult :type Hit%20Result%20Structure%20%28by%20ref%29))
  ;[0 0.000581 0.005] Player got near to this npc. Therefore Npc will start shouting
  (if (Actor|ActorHasTag OtherActor "Actor.Character.Player")
    (Class|GraphNarrationTarget|BeginNarrationGraph (Variables|Default|GetGraphNarrationTarget) (Utilities|Array|MakeArray self) "/Game/_Main/Mechanics/Narration/Graphs/BP_ClerkGreeting.BP_ClerkGreeting_C")))

(event OnInteractionBegin(ClickInteract)
  (params (InteractionActor :type Actor%20Object%20Reference))
  (Class|GraphNarrationTarget|BeginNarrationGraph (Variables|Default|GetGraphNarrationTarget) (Utilities|Array|MakeArray self) "/Game/_Main/Mechanics/Narration/Graphs/BP_ClerkDialogue.BP_ClerkDialogue_C"))

(event Custom|Start%20Shouting
  (Class|GraphNarrationTarget|BeginNarrationGraph (Variables|Default|GetGraphNarrationTarget) (Utilities|Array|MakeArray self) "/Game/_Main/Mechanics/Narration/Graphs/BP_ClerkGreeting.BP_ClerkGreeting_C"))

(event EventBeginPlay
  (|CallParentFunction))

(event Collision|EventActorBeginOverlap
  (params (OtherActor :type Actor%20Object%20Reference))
  (|CallParentFunction OtherActor) ; This node is disabled and will not be called.\nDrag off pins to build functionality.
)

(fn ConstructionScript
  (|CallParentFunction))

(fn OnInteractionEnd
  (params (InteractionTag :type Gameplay%20Tag%20Structure))
  (CallFunction|StartShouting))