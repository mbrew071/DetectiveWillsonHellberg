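; BP_WillsonHellberg is a player character Blueprint with click-to-interact, character outlining and settings menus.
; Left click traces the object under the cursor and asks its ClickInteractComponent to interact unless an interaction is ongoing.
; A looping 0.1-second timer, rather than Tick, feeds the outline trace into SetCharacterOutline.
; Debug keys toggle graphics or input settings widgets, and construction adds the player gameplay tag to actor tags.
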(event Custom|OutlineTick
  ;[0 0.000581 0.005] OutlineTick
  (bind _bshowoutline (CallFunction|TraceOutline))
  (CallFunction|SetCharacterOutline _bshowoutline))

(event Custom|StartOutlineTick
  ;[0 0.000581 0.005] OutlineTick
  (Utilities|Time|SetTimerbyEvent (delegate Custom|OutlineTick) 0.1 true true))

(event EventBeginPlay
  (|CallParentFunction)
  (CallFunction|StartOutlineTick))

(event Collision|EventActorBeginOverlap
  (params (OtherActor :type Actor%20Object%20Reference)))

(event Input|KeyboardEvents|DebugKey1
  (params (Key :type Key%20Structure) (ActionValue :type Input%20Action%20Value%20Structure))
  ;[0 0.000581 0.005] Settings
  (:Pressed
    (bind _settingswidget (Variables|Default|GetSettingsWidget)
      (:then
        (CallFunction|CloseSettingsWIdget _settingswidget)
        (Variables|Default|SetSettingsWidget 0))
      (:else
        (bind _widget (CallFunction|CreateSettingsWidget "/GameSettings/UI/WBP_EgGraphicsSettings.WBP_EgGraphicsSettings_C"))
        (Variables|Default|SetSettingsWidget _widget)))))

(event Input|KeyboardEvents|DebugKey2
  (params (Key :type Key%20Structure) (ActionValue :type Input%20Action%20Value%20Structure))
  ;[0 0.000581 0.005] Settings
  (:Pressed
    (bind _settingswidget (Variables|Default|GetSettingsWidget)
      (:then
        (CallFunction|CloseSettingsWIdget _settingswidget)
        (Variables|Default|SetSettingsWidget 0))
      (:else
        (bind _widget (CallFunction|CreateSettingsWidget "/GameSettings/UI/WBP_EgInputSettings.WBP_EgInputSettings_C"))
        (Variables|Default|SetSettingsWidget _widget)))))

(event Input|MouseEvents|LeftMouseButton
  (params (Key :type Key%20Structure))
  ;[0 0.000581 0.005] Interaction
  (:Pressed
    (bind _actor (CallFunction|GetInteractionActor true))
    (Utilities|IsValid _actor
      (:Is%20Valid
        (CallFunction|InteractwithActor _actor)))))

(fn ConstructionScript
  (|CallParentFunction)
  (CallFunction|InitializeTags))

(fn GetInteractionActor
  (params (bDrawDebug :type Boolean))
  (bind _returnvalue (Game|GetPlayerController 0))
  (bind _array (Utilities|Array|MakeArray "ObjectTypeQuery7"))
  (bind _hitresult (Class|PlayerController|GetHitResultUnderCursorforObjects _returnvalue _array true))
  (bind (_bblockinghit _binitialoverlap _time _distance _location _impactpoint _normal _impactnormal _physmat _hitactor _hitcomponent) (Collision|BreakHitResult _hitresult))
  (Utilities|FlowControl|Sequence
    (:then_0
      (if bDrawDebug
        (Rendering|Debug|DrawDebugSphere _location 1e+01 12 (Utilities|Struct|MakeLinearColor 1.0 0.243137 0.678431 1.0) 0.2 1.0)))
    (:then_1
      (Utilities|IsValid _hitcomponent
        (:Is%20Valid
          (return (Components|GetOwner _hitcomponent)))
        (:Is%20Not%20Valid
          (return _hitactor))))))

(fn InteractwithActor
  (params (ClickedActor :type Actor%20Object%20Reference))
  (bind _output_get (LocalVariables|SetClickInteractCOmponent (Actor|GetComponentbyClass ClickedActor "/Script/ClickInteractionSystem.ClickInteractComponent")))
  ;[0 0.000581 0.005] GetInteractComponent
  (if (not (Variables|/Script/ClickInteractionSystem.ClickInteractComponent|GetbInteractionOngoing _output_get))
    (Utilities|IsValid _output_get
      (:Is%20Valid
        (Class|ClickInteractComponentI|TryInteractwithI(Message) _output_get self))
      (:Is%20Not%20Valid
        _))
    (return)))

(fn InitializeTags
  (Utilities|Array|AddUnique (Variables|Default|GetTags self) (GameplayTags|GetTagName (GameplayTags|MakeLiteralGameplayTag "(TagName=\"Actor.Character.Player\")"))))