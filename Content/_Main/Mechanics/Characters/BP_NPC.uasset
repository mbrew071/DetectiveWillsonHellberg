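; BP_NPC is a non-player character that starts a narration graph when a player click-interacts with it.
; On interaction it saves its yaw, starts the graph on its narration target with both characters as actors, and rotates them to face each other.
; When the graph ends, it breaks both rotations, restores only its own yaw and ends the interaction.
; A missing target or failed start ends the interaction as unsuccessful.
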(event OnInteractionBegin(ClickInteract)
  (params (InteractionActor :type Actor%20Object%20Reference))
  (bind _self self)
  (bind _self_2 self)
  (bind _graphnarrationtarget (Variables|Default|GetGraphNarrationTarget))
  (bind _returnvalue (Transformation|GetActorLocation _self_2))
  (Variables|Default|SetInteractingCharacter InteractionActor)
  (Utilities|IsValid _graphnarrationtarget
    (:Is%20Valid
      (bind _npc (CallFunction|GetInitialRotations self))
      (bind _returnvalue_2 (Class|GraphNarrationTarget|BeginNarrationGraph _graphnarrationtarget (Utilities|Array|MakeArray (Variables|Default|GetInteractingCharacter) self) 0 (delegate Custom|CustomEvent)))
      (if _returnvalue_2
        (Utilities|FlowControl|Sequence
          (:then_0
            ;[0 0.000581 0.005] Rotate player towards NPC
            (Utilities|ZRotateActor 1.0 (Variables|Default|GetInteractingCharacter) (.yaw (Transformation|GetActorRotation (Variables|Default|GetInteractingCharacter))) (.yaw (Math|Rotator|FindLookatRotation (Transformation|GetActorLocation (Variables|Default|GetInteractingCharacter)) _returnvalue))))
          (:then_1
            ;[0 0.000581 0.005] Rotate NPC towards player
            (Utilities|ZRotateActor 1.0 _self (.yaw (Transformation|GetActorRotation _self)) (.yaw (Math|Rotator|FindLookatRotation _returnvalue (Transformation|GetActorLocation (Variables|Default|GetInteractingCharacter)))))))
        (else
          (Default|CallOnInteractionEnd (Variables|Default|GetClickInteract) false))))
    (:Is%20Not%20Valid
      (Default|CallOnInteractionEnd (Variables|Default|GetClickInteract) false))))

(event Custom|CustomEvent
  (bind _self self)
  (bind _self_2 self)
  (bind _self_3 self)
  (bind _interactingcharacter (Variables|Default|GetInteractingCharacter))
  (bind _interactingcharacter_2 (Variables|Default|GetInteractingCharacter))
  (bind _returnvalue (Transformation|GetActorLocation _self_3))
  (bind _returnvalue_2 (Transformation|GetActorLocation _interactingcharacter_2))
  (bind _returnvalue_3 (Transformation|GetActorRotation _self_2))
  (Utilities|FlowControl|Sequence
    (:then_0
      ;[0 0.000581 0.005] Make sure it finished previous rotation
      (Utilities|FlowControl|Sequence
        (:then_0
          ;[0 0.000581 0.005] Rotate player towards NPC
          (Utilities|ZRotateActor 1.0 _interactingcharacter (.yaw (Transformation|GetActorRotation _interactingcharacter)) (.yaw (Math|Rotator|FindLookatRotation _returnvalue_2 _returnvalue))) ; enters at Break
        )
        (:then_1
          ;[0 0.000581 0.005] Rotate NPC towards player
          (Utilities|ZRotateActor 1.0 _self (.yaw (Transformation|GetActorRotation _self)) (.yaw (Math|Rotator|FindLookatRotation _returnvalue _returnvalue_2))) ; enters at Break
        )))
    (:then_1
      ;[0 0.000581 0.005] Revert rotations
      (Transformation|SetActorRotation _self_2 (Math|Rotator|MakeRotator (.roll _returnvalue_3) (.pitch _returnvalue_3) (stale OnInteractionBegin(ClickInteract) _npc)))
      (Default|CallOnInteractionEnd (Variables|Default|GetClickInteract) true))))

(event EventBeginPlay
  (|CallParentFunction) ; This node is disabled and will not be called.\nDrag off pins to build functionality.
)

(fn ConstructionScript
  (|CallParentFunction))

(fn GetInitialRotations
  (params (CharB :type Actor%20Object%20Reference))
  (return (.yaw (Transformation|GetActorRotation CharB))))

(fn OnInteractionBegin)