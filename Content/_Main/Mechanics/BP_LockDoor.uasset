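; BP_LockDoor is a lockable physics door that alternates between free-swinging and locked each time FlipFlopLock is called.
; Unlocking stops any closing timer and turns on physics simulation on the Door component.
; Locking disables physics and starts a looping timer that eases the door's relative yaw back to zero with FInterpTo, clearing itself once nearly closed.
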(event Custom|Tick
  (bind _returnvalue (Math|Float|MakeLiteralFloat 0.0))
  (bind _door (Variables|Default|GetDoor))
  (bind _relativerotation (Variables|/Script/Engine.SceneComponent|GetRelativeRotation _door))
  (Transformation|SetRelativeRotation (Variables|Default|GetDoor) (Math|Rotator|MakeRotator (.roll _relativerotation) (.pitch _relativerotation) (Math|Interpolation|FInterpTo (.yaw _relativerotation) _returnvalue (Utilities|Time|GetWorldDeltaSeconds) 1e+01)) true false)
  (if (Math|Float|NearlyEqual(Float) (.yaw (Variables|/Script/Engine.SceneComponent|GetRelativeRotation (Variables|Default|GetDoor))) _returnvalue 0.001)
    (Utilities|Time|ClearandInvalidateTimerbyHandle (stale Custom|FlipFlopLock _returnvalue))))

(event Custom|FlipFlopLock
  (Utilities|FlowControl|FlipFlop
    (:A
      ;[0 0.000581 0.005] OpenLock
      (Utilities|Time|ClearandInvalidateTimerbyHandle (stale _returnvalue))
      (Physics|SetSimulatePhysics (Variables|Default|GetDoor) true))
    (:B
      ;[0 0.000581 0.005] Close Lock
      (Physics|SetSimulatePhysics (Variables|Default|GetDoor) false)
      (bind _returnvalue (Utilities|Time|SetTimerbyEvent (delegate Custom|Tick) 0.02 true)))))

(event EventBeginPlay
  (|CallParentFunction) ; This node is disabled and will not be called.\nDrag off pins to build functionality.
)

(event Collision|EventActorBeginOverlap
  (params (OtherActor :type Actor%20Object%20Reference))
  (|CallParentFunction OtherActor) ; This node is disabled and will not be called.\nDrag off pins to build functionality.
)

(event EventTick
  (params (DeltaSeconds :type Float%20%28single-precision%29))
  (|CallParentFunction DeltaSeconds))

(fn ConstructionScript
  (|CallParentFunction))