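; BP_Door is a door that swings between an open angle and an initial angle each time TriggerDoor is called.
; TriggerDoor flip-flops the target yaw and starts a looping timer that drives DoorTick in place of Tick.
; DoorTick eases the Door component's yaw toward the target with a swept interpolation, then clears the timer when nearly there.
; Logic to toggle the door's collision during movement is present but disconnected.
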(event Custom|TriggerDoor
  (bind _isa (Utilities|FlowControl|FlipFlop)
    (:A
      (Variables|Default|SetTarget (Variables|Default|GetOpenAngle)))
    (:B
      (Variables|Default|SetTarget (Variables|Default|GetInitialAngle))))
  (bind _returnvalue (Utilities|Time|SetTimerbyEvent (delegate Custom|DoorTick) 0.02 true)))

(event Custom|DoorTick
  (bind _door (Variables|Default|GetDoor))
  (bind _relativerotation (Variables|/Script/Engine.SceneComponent|GetRelativeRotation _door))
  (Transformation|SetRelativeRotation (Variables|Default|GetDoor) (Math|Rotator|MakeRotator (.roll _relativerotation) (.pitch _relativerotation) (Math|Interpolation|FInterpTo (.yaw _relativerotation) (Variables|Default|GetTarget) (Utilities|Time|GetWorldDeltaSeconds) 8.0)) true false)
  (if (Math|Float|NearlyEqual(Float) (.yaw (Variables|/Script/Engine.SceneComponent|GetRelativeRotation (Variables|Default|GetDoor))) (Math|Float|SelectFloat (Variables|Default|GetOpenAngle) (Variables|Default|GetTarget) (stale Custom|TriggerDoor _isa)) 0.1)
    (Utilities|Time|ClearandInvalidateTimerbyHandle (stale Custom|TriggerDoor _returnvalue))))

(event EventBeginPlay)

(event Collision|EventActorBeginOverlap
  (params (OtherActor :type Actor%20Object%20Reference)))

(event EventTick
  (params (DeltaSeconds :type Float%20%28single-precision%29)))

(fn ConstructionScript)