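; BP_ShopEnter is an interactable shop entrance that sends the game to the Shop world.
; Its Trigger overlap sets an in-range flag for any actor, but shows or hides the interact prompt widget only for the player character.
; Releasing E while in range asks the LevelChangeManager to start a non-automatic world transition.
; EnableInput is called inside that key handler rather than at BeginPlay.
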(event OnComponentBeginOverlap(Trigger)
  (params (OverlappedComponent :type Primitive%20Component%20Object%20Reference) (OtherActor :type Actor%20Object%20Reference) (OtherComp :type Primitive%20Component%20Object%20Reference) (OtherBodyIndex :type Integer) (bFromSweep :type Boolean) (SweepResult :type Hit%20Result%20Structure%20%28by%20ref%29))
  (Variables|Default|SetIs%20in%20Range true)
  (if (== OtherActor (Game|GetPlayerCharacter 0))
    (UserInterface|Viewport|AddtoViewport (Variables|Default|GetInteract%20Prompt) 0)))

(event OnComponentEndOverlap(Trigger)
  (params (OverlappedComponent :type Primitive%20Component%20Object%20Reference) (OtherActor :type Actor%20Object%20Reference) (OtherComp :type Primitive%20Component%20Object%20Reference) (OtherBodyIndex :type Integer))
  (Variables|Default|SetIs%20in%20Range false)
  (if (== OtherActor (Game|GetPlayerCharacter 0))
    (Widget|RemovefromParent (Variables|Default|GetInteract%20Prompt))))

(event EventBeginPlay
  (bind _returnvalue (UserInterface|CreateWidget "/Game/_Main/UI/InteractWidget.InteractWidget_C"))
  (Variables|Default|SetInteract%20Prompt _returnvalue))

(event Input|KeyboardEvents|E
  (params (Key :type Key%20Structure :default "None"))
  (:Released
    (Input|EnableInput 0)
    (if (Variables|Default|GetIs%20in%20Range)
      (Class|LevelChangeManager|StartWorldTransition (Subsystems|GetLevelChangeManager) "/Game/_Main/Levels/ClosedLocations/Shop.Shop" false 0.0))))

(fn ConstructionScript)