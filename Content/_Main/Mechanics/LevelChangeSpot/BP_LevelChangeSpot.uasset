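; BP_LevelChangeSpot is an interactable spot that moves the game to a target level when its ClickInteract component begins an interaction.
; It passes PlayerStartTag as a level option to select the arrival point.
; With the editor it opens the world directly by reference, otherwise it routes through LevelChangeManager with auto-transition and delay settings.
; It then signals the end of the interaction.
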(event OnInteractionBegin(ClickInteract)
  (params (InteractionActor :type Actor%20Object%20Reference))
  (bind _playerstarttag (Variables|Design|GetPlayerStartTag))
  (bind _returnvalue (Utilities|String|Append "PlayerStartTag=" _playerstarttag))
  (if (Class|LowEntryExtendedStandardLibrary|WithEditor)
    (Game|OpenLevel(byObjectReference) (Variables|Design|GetTargetWorld) true _returnvalue)
    (else
      (Class|LevelChangeManager|OpenLevel(byName) (Subsystems|GetLevelChangeManager) (Variables|Design|GetTargetWorld) (Variables|Design|GetIn%20Auto%20Transition) (Variables|Design|GetAutoTransitionDelay) _returnvalue)))
  (Default|CallOnInteractionEnd (Variables|Default|GetClickInteract) true))

(fn ConstructionScript)