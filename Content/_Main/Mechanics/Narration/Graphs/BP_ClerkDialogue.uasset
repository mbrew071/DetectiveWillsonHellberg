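; Narration graph for a shop clerk's dialogue, with Polish text.
; On begin it shows two options through an async display action: a shop remark and a greeting.
; The shop option plays two screen narration lines from the clerk, then lists the options again.
; The greeting starts a farewell line and ends the graph without waiting for it, and failures in the options or shop narration also end it.
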(event Custom|ListMainOptions
  (bind _chosenoption (Class|NarrationGraph|ActionDisplayOptions (Utilities|Array|MakeArray (Utilities|Struct|MakeNarrationOption "Sklep..." true "DefaultOptionSecondary") (Utilities|Struct|MakeNarrationOption "Elo" true "DefaultOptionSecondary")))
    (:Completed
      (switch int _chosenoption
        (:0
          (Class|NarrationGraph|ActionPlayScreenNarration (Utilities|Array|MakeArray (Utilities|Struct|MakeScreenNarrationPiece "Sprzedawca" "Może i nie jest tu zbyt tanio") (Utilities|Struct|MakeScreenNarrationPiece "Sprzedawca" "ale za to pachnie starociami"))
            (:Completed
              (CallFunction|ListMainOptions))
            (:Failed
              (Class|NarrationGraph|ActionEndGraph))))
        (:1
          (Class|NarrationGraph|ActionPlayScreenNarration (Utilities|Array|MakeArray (Utilities|Struct|MakeScreenNarrationPiece "Sprzedawca" "Bywaj"))
            (:Completed
              _)
            (:Failed
              _))
          (Class|NarrationGraph|ActionEndGraph))))
    (:Failed
      (Class|NarrationGraph|ActionEndGraph))))

(event EventBeginGraph
  (bind _chosenoption (Class|NarrationGraph|ActionDisplayOptions (Utilities|Array|MakeArray (Utilities|Struct|MakeNarrationOption "Sklep..." true "DefaultOptionSecondary") (Utilities|Struct|MakeNarrationOption "Elo" true "DefaultOptionSecondary")))
    (:Completed
      (switch int _chosenoption
        (:0
          (Class|NarrationGraph|ActionPlayScreenNarration (Utilities|Array|MakeArray (Utilities|Struct|MakeScreenNarrationPiece "Sprzedawca" "Może i nie jest tu zbyt tanio") (Utilities|Struct|MakeScreenNarrationPiece "Sprzedawca" "ale za to pachnie starociami"))
            (:Completed
              (CallFunction|ListMainOptions))
            (:Failed
              (Class|NarrationGraph|ActionEndGraph))))
        (:1
          (Class|NarrationGraph|ActionPlayScreenNarration (Utilities|Array|MakeArray (Utilities|Struct|MakeScreenNarrationPiece "Sprzedawca" "Bywaj"))
            (:Completed
              _)
            (:Failed
              _))
          (Class|NarrationGraph|ActionEndGraph))))
    (:Failed
      (Class|NarrationGraph|ActionEndGraph))))