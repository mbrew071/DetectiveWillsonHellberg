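; Narration graph in which a shop clerk, labelled "Sprzedawca", greets with Polish voice lines or text through scene narration on the first narration actor.
; After a short delay it plays a fixed welcome, then on completion waits briefly and starts one of three randomly selected follow-up phrases.
; The graph end is called right after starting the follow-up, without waiting for its completion, or immediately if the welcome fails.
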(event EventBeginGraph
  (Utilities|FlowControl|Delay 2.0)
  (Class|NarrationGraph|ActionPlaySceneNarration (.Actor (Class|NarrationGraph|GetNarrationActorPure)) (Utilities|Array|MakeArray (Utilities|Struct|MakeSceneNarrationPiece "Sprzedawca" "Witaj w moim sklepie"))
    (:Completed
      (Utilities|FlowControl|Delay 1.0)
      (Class|NarrationGraph|ActionPlaySceneNarration (.Actor (Class|NarrationGraph|GetNarrationActorPure)) (Utilities|Array|MakeArray (Utilities|Struct|MakeSceneNarrationPiece "Sprzedawca" (Utilities|Select :Index (Math|Random|RandomIntegerinRange 0 2) :Option%200 "Smialo rozejrzyj sie" :Option%201 "Jestem pewny ze cos przypadnie ci do gustu" :Option%202 "W czym mogę ci pomoc?")))
        (:Completed
          _)
        (:Failed
          _))
      (Class|NarrationGraph|ActionEndGraph))
    (:Failed
      (Class|NarrationGraph|ActionEndGraph))))