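; Game instance for the detective game that sets up the game settings and level change plugins when it starts.
; The settings controller receives Blueprint classes for graphics and input bindings and a JSON path in the project's Saved directory, then applies example default settings.
; The level change manager is initialized with WBP_Transition as its transition widget.
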(event EventStart
  (CallFunction|InitGameSettings)
  (CallFunction|InitLevelChanger))

(fn InitGameSettings
  (bind (_bool _int _float _input) (CallFunction|GetExampleDefaultSettings))
  (Class|GameSettingsController|InitializePlugin (Subsystems|GetGameSettingsController) "/GameSettings/SettingsControllers/BP_GraphicsSettingsController.BP_GraphicsSettingsController_C" 0 0 "/GameSettings/SettingsControllers/BP_InputSettingsController.BP_InputSettingsController_C" (CallFunction|GetExampleJsonSerializedSettings) (Class|BlueprintPathsLibrary|ProjectSavedDir) (Utilities|Set|MakeSet))
  (bind _returnvalue (Class|GameSettingsController|InitializeSettings (Subsystems|GetGameSettingsController) _bool _int _float _input))
  (if _returnvalue
    _))

(fn InitLevelChanger
  (bind _returnvalue (Class|LevelChangeManager|InitializePlugin (Subsystems|GetLevelChangeManager) "/Game/_Main/UI/TransitionWIdget/WBP_Transition.WBP_Transition_C"))
  (if _returnvalue
    _))