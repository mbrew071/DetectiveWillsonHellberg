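; BP_DetectiveGameMode is a game mode Blueprint that decides where a player spawns in the level.
; It overrides ChoosePlayerStart to return the PlayerStart whose tag matches the PlayerStartTag option in the game mode's options string, so the spawn point can be set through travel options.
; When no tag matches, it falls back to the last PlayerStart found.
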(fn ConstructionScript)

(fn ChoosePlayerStart
  (params (Player :type Controller%20Object%20Reference))
  (bind _outactors (Actor|GetAllActorsOfClass "/Script/Engine.PlayerStart"))
  (for _array_element _outactors
    (if (== (Variables|/Script/Engine.PlayerStart|GetPlayerStartTag _array_element) (Class|GameplayStatics|ParseOption (Variables|Default|GetOptionsString) "PlayerStartTag"))
      (return _array_element)))
  (return (Utilities|Array|Get(acopy) _outactors (Utilities|Array|LastIndex _outactors))))